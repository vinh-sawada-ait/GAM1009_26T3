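; BP_PickUp is a collectible actor that homes in on the actor entering its sphere, then hands over its properties and destroys itself.
; A sphere overlap triggers a one-shot activation that plays the MoveToPlayer timeline, lerping from the pickup's current location toward the target's live location each update.
; When the timeline finishes, it sends PickUpProperties through ActivatePickUpAttributesMessage and runs the collected sequence, which only destroys the actor.
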(event OnComponentBeginOverlap(Sphere)
  (params (OverlappedComponent :type Primitive%20Component%20Object%20Reference) (OtherActor :type Actor%20Object%20Reference) (OtherComp :type Primitive%20Component%20Object%20Reference) (OtherBodyIndex :type Integer) (bFromSweep :type Boolean) (SweepResult :type Hit%20Result%20Structure%20%28by%20ref%29))
  (CallFunction|ActivatePickUpHoming OtherActor))

(event Custom|PickUpCollectedSequence
  (Actor|DestroyActor))

(event EventActivatePickUpHoming
  (params (PlayerPawn :type Actor%20Object%20Reference))
  (Utilities|FlowControl|DoOnce false
    (:Completed
      (bind _alpha (Timeline|MoveToPlayer Play)
        (:Update
          (Transformation|SetActorLocation (Math|Vector|Lerp(Vector) (Transformation|GetActorLocation) (Transformation|GetActorLocation PlayerPawn) _alpha) false false))
        (:Finished
          ;[1 0 0 0.5] Needs attribute values sent
          (Class|BPIMyFlyingShmup|ActivatePickUpAttributes(Message) PlayerPawn (Variables|Default|GetPickUpProperties))
          (CallFunction|PickUpCollectedSequence))))))

(fn ConstructionScript)