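; BP_Turret is an enemy turret that fires projectiles at regular intervals.
; A looping timer started on BeginPlay spawns an enemy bullet at the Arrow component's transform and plays a gunshot sound while ShootingEnabled is true.
; With AutoAim on, Tick yaws the Cylinder component toward player 0's pawn using a look-at rotation, with no range or line-of-sight check.
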(event Custom|ShootBullet
  (bind _arrow (Variables|Default|GetArrow))
  ;[0.15 0.15 0.15 0.5] Shoot Bullet
  (if (Variables|Default|GetShootingEnabled)
    (Game|SpawnActorfromClass "/Game/Blueprints/BP_Projectile_Bullet_Enemy.BP_Projectile_Bullet_Enemy_C" (Math|Transform|MakeTransform (Transformation|GetWorldLocation _arrow) (Transformation|GetWorldRotation _arrow) "1.000000,1.000000,1.000000") "Undefined" "MultiplyWithRoot" 0 0)
    (Audio|PlaySound2D "/Game/FreeWeaponSFX/Cue/Handgun/Gunshots/sfx_wpn_hgn_gunshot_01_Cue.sfx_wpn_hgn_gunshot_01_Cue" 1.0 1.0 0.0 0 0)))

(event EventBeginPlay
  (Utilities|Time|SetTimerbyEvent (delegate Custom|ShootBullet) 2.0 true true))

(event EventTick
  (params (DeltaSeconds :type Float%20%28single-precision%29))
  (bind _returnvalue (Game|Player|GetPlayerPawn 0))
  (Utilities|IsValid _returnvalue
    (:Is%20Valid
      (if (Variables|Default|GetAutoAim)
        (Transformation|SetWorldRotation (Variables|Default|GetCylinder) (Math|Rotator|MakeRotator 0.0 0.0 (.yaw (Math|Rotator|FindLookatRotation (Transformation|GetActorLocation) (Transformation|GetActorLocation _returnvalue)))) false false)))))

(fn ConstructionScript)