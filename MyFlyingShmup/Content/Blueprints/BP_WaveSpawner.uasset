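; Wave spawner actor that spawns timed waves of enemies from a waves data asset, starting on BeginPlay.
; Three chained events step through waves, enemy sets and individual spawns using index counters and Delays, advancing without waiting for enemies to die.
; Each set's initial delay also spaces its individual spawns.
; Regular enemies spawn at a random Y offset from the spawner, while boss waves use a fixed world location.
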(event Custom|SpawnWave
  (bind _wavesdataasset (Variables|Default|GetWavesDataAsset))
  (bind _currentwaveid (Variables|Default|GetCurrentWaveId))
  (bind _waves (Variables|/Game/Core/PDA_SetOfWaves.PDA_SetOfWaves_C|GetWaves _wavesdataasset))
  (bind _output (Utilities|Array|Get(acopy) _waves _currentwaveid))
  ;[0.15 0.15 0.15 0.5] Spawn Wave 1, Wave 2, Wave 3
  (if (Utilities|Array|IsValidIndex (Variables|/Game/Core/PDA_SetOfWaves.PDA_SetOfWaves_C|GetWaves (Variables|Default|GetWavesDataAsset)) (Variables|Default|GetCurrentWaveId))
    (Variables|Default|SetCurrentEnemiesInWaveData (.enemiesinwave _output))
    (Variables|Default|SetisBoss (.isboss _output))
    (Utilities|FlowControl|Delay (.initialdelayforwave _output))
    (Variables|Default|SetCurrentEnemiesInWave 0)
    (CallFunction|SpawnEnemiesinWave)
    (Development|PrintString "Spawn Wave")
    (else
      (Development|PrintString "All Waves have finished"))))

(event Custom|SpawnEnemiesInWave
  ;[0.15 0.15 0.15 0.5] Spawn Enemy Set 1, Enemy Set 2, Enemy Set 3
  (if (Utilities|Array|IsValidIndex (Variables|Default|GetCurrentEnemiesInWaveData) (Variables|Default|GetCurrentEnemiesInWave))
    (Utilities|FlowControl|Delay (.initialdelayuntilspawn (Utilities|Array|Get(acopy) (Variables|Default|GetCurrentEnemiesInWaveData) (Variables|Default|GetCurrentEnemiesInWave))))
    (Variables|Default|SetCurrentSpawnCount 0)
    (CallFunction|SpawnEnemy)
    (Development|PrintString "Spawn Next Enemy Set")
    (else
      (Math|Integer|IncrementInt (Variables|Default|GetCurrentWaveId)
        (:%20%20
          (CallFunction|SpawnWave))))))

(event Custom|SpawnEnemy
  (bind _currentenemiesinwave (Variables|Default|GetCurrentEnemiesInWave))
  (bind _currentenemiesinwavedata (Variables|Default|GetCurrentEnemiesInWaveData))
  (bind _output (Utilities|Array|Get(acopy) _currentenemiesinwavedata _currentenemiesinwave))
  ;[0.15 0.15 0.15 0.5] Spawn Enemy Type
  (if (>= (Variables|Default|GetCurrentSpawnCount) (.spawncount _output))
    (Math|Integer|IncrementInt (Variables|Default|GetCurrentEnemiesInWave)
      (:%20%20
        (CallFunction|SpawnEnemiesinWave)))
    (else
      (Utilities|FlowControl|Delay (.initialdelayuntilspawn _output))
      (Game|SpawnActorfromClass (.enemyclass _output) (Math|Transform|MakeTransform (select (Variables|Default|GetisBoss) "3000.000000,0.000000,800.000000" (+ (Transformation|GetActorLocation) (Math|Vector|MakeVector 0.0 (Math|Random|RandomFloatinRange -2e+03 2e+03) 0.0))) (Transformation|GetActorRotation) "1.000000,1.000000,1.000000") "AlwaysSpawn" "MultiplyWithRoot" 0 0)
      (Math|Integer|IncrementInt (Variables|Default|GetCurrentSpawnCount)
        (:%20%20
          (Development|PrintString "Spawn enemy")
          (CallFunction|SpawnEnemy))))))

(event EventBeginPlay
  (CallFunction|SpawnWave))

(fn ConstructionScript)