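; Enemy actor with a health widget that deals its remaining Health as damage to whatever overlaps it.
; On BeginPlay it may randomly spawn an attached BP_Turret with random auto-aim.
; Damage flashes a white overlay, plays a sound, updates health, and awards score to the instigator with a screen-projected popup.
; At zero health it awards MaxHealth as bonus score, spawns an explosion, and destroys itself and its turret.
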(event Custom|DeathSequence
  ;[0.15 0.15 0.15 0.5] Death Sequence
  (CallFunction|ApplyDamageasScore (Variables|Default|GetMaxHealth))
  (Audio|PlaySound2D "/Game/FreeWeaponSFX/Cue/GrenadeLauncher/sfx_wpn_gl_explosion_Cue.sfx_wpn_gl_explosion_Cue" 1.0 1.0 0.0 0 0)
  (Game|SpawnActorfromClass "/Game/VFX/BP_Explosion.BP_Explosion_C" (Math|Transform|MakeTransform (Transformation|GetActorLocation) (Transformation|GetActorRotation) "1.000000,1.000000,1.000000") "Undefined" "MultiplyWithRoot" 0 0)
  ;;[0.15 0.15 0.15 0.5] Destory turrent if valid
  (bind _turret (Variables|Default|GetTurret)
    (:then
      (Actor|DestroyActor _turret))
    (:else
      _))
  (Actor|DestroyActor))

(event Custom|HitSequence
  ;[0.15 0.15 0.15 0.5] Hit Sequence
  (Audio|PlaySound2D "/Game/FreeWeaponSFX/Cue/Handgun/Gunshots/sfx_wpn_hgn_gunshot_01_Cue.sfx_wpn_hgn_gunshot_01_Cue" 1.0 1.0 0.0 0 0)
  (Rendering|Material|SetOverlayMaterial (Variables|Default|GetStaticMesh) "/Game/Materials/MI_Overly_HitEffect_White.MI_Overly_HitEffect_White" false 0 :!class /Script/Engine.MeshComponent)
  (Utilities|FlowControl|Delay 0.2)
  (Rendering|Material|SetOverlayMaterial (Variables|Default|GetStaticMesh) 0 false 0 :!class /Script/Engine.MeshComponent))

(event Custom|SetWidgetHealth
  ;[0.15 0.15 0.15 0.5] Widget Health
  (Class|BPIMyFlyingShmup|SetHealth(Message) (UserInterface|GetUserWidgetObject (Variables|Default|GetWidget)) (Math|Float|SafeDivide (Variables|Default|GetHealth) (Variables|Default|GetMaxHealth)) (Variables|Default|GetHealth)))

(event Custom|ApplyDamageAsScore
  (params (Points :type Float%20%28double-precision%29))
  (bind _instigatedby (Variables|Default|GetInstigatedBy)
    (:then
      (Class|BPIMyFlyingShmup|AddScore(Message) _instigatedby Points)
      (bind _returnvalue (UserInterface|CreateWidget "/Game/Ui/W_DamagePopUp.W_DamagePopUp_C" (.AsPlayer%20Controller (Utilities|Casting|CastToPlayerController _instigatedby))))
      (UserInterface|Viewport|AddtoViewport _returnvalue 0)
      (Class|UserWidget|SetPositioninViewport _returnvalue (.ScreenPosition (Class|WidgetLayoutLibrary|ProjectWorldLocationtoWidgetPosition (Game|GetPlayerController 0) (Transformation|GetActorLocation) false)) false))
    (:else)))

(event Custom|SpawnRandomTurret
  ;[0.15 0.15 0.15 0.5] Randomly spawn and attach the turret
  (if (< (Math|Random|RandomFloat) 0.2)
    (bind _returnvalue (Game|SpawnActorfromClass "/Game/Blueprints/BP_Turret.BP_Turret_C" (Math|Transform|MakeTransform "0, 0, 0" "0, 0, 0" "1.000000,1.000000,1.000000") "AlwaysSpawn" "MultiplyWithRoot" 0 (Math|Random|RandomBool) 0))
    (bind _output_get (Variables|Default|SetTurret _returnvalue))
    (Transformation|AttachComponentToComponent _output_get (Variables|Default|GetTurrentAttachPoint) "None" "KeepRelative" "KeepRelative" "KeepRelative" false)))

(event Collision|EventActorBeginOverlap
  (params (OtherActor :type Actor%20Object%20Reference))
  (Game|Damage|ApplyDamage OtherActor (Variables|Default|GetHealth) 0 0))

(event Game|Damage|EventAnyDamage
  (params (Damage :type Float%20%28single-precision%29) (DamageType :type Damage%20Type%20Object%20Reference) (InstigatedBy :type Controller%20Object%20Reference) (DamageCauser :type Actor%20Object%20Reference))
  ;[0.15 0.15 0.15 0.5] Damage and Health calculation
  (Variables|Default|SetInstigatedBy InstigatedBy)
  (CallFunction|ApplyDamageasScore Damage)
  (CallFunction|HitSequence)
  (bind _output_get (Variables|Default|SetHealth (Math|Float|Max(Float) (- (Variables|Default|GetHealth) Damage) 0.0)))
  (CallFunction|SetWidgetHealth)
  (if (== _output_get 0.0)
    (Utilities|FlowControl|DelayUntilNextFrame)
    (CallFunction|DeathSequence)))

(event EventBeginPlay
  (Variables|Default|SetHealth (Variables|Default|GetMaxHealth))
  (CallFunction|SetWidgetHealth)
  (CallFunction|SpawnRandomTurret))

(fn ConstructionScript)