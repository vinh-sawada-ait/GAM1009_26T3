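; First boss enemy, an actor carrying six BP_Turret child actors as its weapons.
; On BeginPlay it runs the parent logic and switches off shooting on every turret.
; After a short delay it activates MoveSideToSide and re-enables shooting on all turrets.
; SpawnRandomTurret is an empty event, and the Tick and overlap events do nothing.
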(event EventBeginPlay
  (bind _childactor1 (Variables|Default|GetChildActor1))
  (bind _childactor3 (Variables|Default|GetChildActor3))
  (bind _childactor4 (Variables|Default|GetChildActor4))
  (bind _childactor5 (Variables|Default|GetChildActor5))
  (bind _childactor (Variables|Default|GetChildActor))
  (bind _childactor2 (Variables|Default|GetChildActor2))
  (bind _array (Utilities|Array|MakeArray _childactor1 _childactor3 _childactor4 _childactor5 _childactor _childactor2))
  (|CallParentFunction)
  (for _array_element _array
    (bind _asbp_turret (Utilities|Casting|CastToBP_Turret (Variables|/Script/Engine.ChildActorComponent|GetChildActor _array_element)))
    (Variables|/Game/Blueprints/BP_Turret.BP_Turret_C|SetShootingEnabled _asbp_turret false))
  (Utilities|FlowControl|Delay 5.0)
  (Components|Activation|Activate (Variables|Default|GetMoveSideToSide) false)
  (for _array_element_2 _array
    (bind _asbp_turret_2 (Utilities|Casting|CastToBP_Turret (Variables|/Script/Engine.ChildActorComponent|GetChildActor _array_element_2)))
    (Variables|/Game/Blueprints/BP_Turret.BP_Turret_C|SetShootingEnabled _asbp_turret_2 true)))

(event Collision|EventActorBeginOverlap
  (params (OtherActor :type Actor%20Object%20Reference))
  (|CallParentFunction OtherActor) ; This node is disabled and will not be called.\nDrag off pins to build functionality.
)

(event EventTick
  (params (DeltaSeconds :type Float%20%28single-precision%29)))

(event EventSpawnRandomTurret)

(fn ConstructionScript
  (|CallParentFunction))