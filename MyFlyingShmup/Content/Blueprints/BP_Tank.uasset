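; Player-drivable tank actor that takes keyboard input from player 0 to move, turn and rotate its turret.
; W/S, A/D and Q/E each open a Gate while held, and a Tick Sequence feeds all six Gates.
; Open Gates apply fixed per-frame offsets without delta time, sweeping forward and backward movement for collision.
; Wheels spin with movement and counter-rotate by pair during turns, while the Head rotates independently.
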(event EventBeginPlay
  ;[1 0.46 0 0.5] Enable Inputs for Player 0
  (Input|EnableInput (Game|GetPlayerController 0)))

(event EventTick
  (params (DeltaSeconds :type Float%20%28single-precision%29))
  (bind _head (Variables|Default|GetHead))
  (bind _wheel2 (Variables|Default|GetWheel2))
  (Utilities|FlowControl|Sequence
    (:then_0
      ;[0.15 1 0.15 0.5] Move Forward and Backwards
      (Utilities|FlowControl|Gate true
        (:Exit
          (Transformation|AddActorLocalOffset "1.000000,0.000000,0.000000" true false)
          ;[0.7913 0.6087 0 0.5] Rotate Wheel when moving
          (Transformation|AddLocalRotation _wheel2 "-2.000000,0.000000,0.000000" false false))))
    (:then_1
      (Utilities|FlowControl|Gate true
        (:Exit
          (Transformation|AddActorLocalOffset "-1.000000,0.000000,0.000000" true false)
          (Transformation|AddLocalRotation _wheel2 "2.000000,0.000000,0.000000" false false))))
    (:then_2
      ;[0.15 1 0.15 0.5] Rotate Entire Tank
      (Utilities|FlowControl|Gate true
        (:Exit
          (Transformation|AddActorLocalRotation "0.000000,-1.000000,0.000000" false false)
          ;[0.7913 0.6087 0 0.5] Rotate Wheels when tank rotated
          (Transformation|AddLocalRotation (Variables|Default|GetWheel2) "-1.000000,0.000000,0.000000" false false)
          (Transformation|AddLocalRotation (Variables|Default|GetWheel3) "1.000000,0.000000,0.000000" false false))))
    (:then_3
      (Utilities|FlowControl|Gate true
        (:Exit
          (Transformation|AddActorLocalRotation "0.000000,1.000000,0.000000" false false)
          (Transformation|AddLocalRotation (Variables|Default|GetWheel2) "1.000000,0.000000,0.000000" false false)
          (Transformation|AddLocalRotation (Variables|Default|GetWheel3) "-1.000000,0.000000,0.000000" false false))))
    (:then_4
      ;[0.15 1 0.15 0.5] Rotate Head/Turret/Canon
      (Utilities|FlowControl|Gate true
        (:Exit
          (Transformation|AddLocalRotation _head "0.000000,-1.000000,0.000000" false false))))
    (:then_5
      (Utilities|FlowControl|Gate true
        (:Exit
          (Transformation|AddLocalRotation _head "0.000000,1.000000,0.000000" false false))))))

(event Input|KeyboardEvents|E
  (params (Key :type Key%20Structure :default "None"))
  ;[0.15 1 0.15 0.5] Rotate Head/Turret/Canon
  (:Pressed
    (Utilities|FlowControl|Gate true) ; enters at Open
  )
  (:Released
    (Utilities|FlowControl|Gate true) ; enters at Close
  ))

(event Input|KeyboardEvents|Q
  (params (Key :type Key%20Structure :default "None"))
  ;[0.15 1 0.15 0.5] Rotate Head/Turret/Canon
  (:Pressed
    (Utilities|FlowControl|Gate true) ; enters at Open
  )
  (:Released
    (Utilities|FlowControl|Gate true) ; enters at Close
  ))

(event Input|KeyboardEvents|W
  (params (Key :type Key%20Structure :default "None"))
  ;[0.15 1 0.15 0.5] Move Forward and Backwards
  (:Pressed
    (Utilities|FlowControl|Gate true) ; enters at Open
  )
  (:Released
    (Utilities|FlowControl|Gate true) ; enters at Close
  ))

(event Input|KeyboardEvents|S
  (params (Key :type Key%20Structure :default "None"))
  ;[0.15 1 0.15 0.5] Move Forward and Backwards
  (:Pressed
    (Utilities|FlowControl|Gate true) ; enters at Open
  )
  (:Released
    (Utilities|FlowControl|Gate true) ; enters at Close
  ))

(event Input|KeyboardEvents|A
  (params (Key :type Key%20Structure :default "None"))
  ;[0.15 1 0.15 0.5] Rotate Entire Tank
  (:Pressed
    (Utilities|FlowControl|Gate true) ; enters at Open
  )
  (:Released
    (Utilities|FlowControl|Gate true) ; enters at Close
  ))

(event Input|KeyboardEvents|D
  (params (Key :type Key%20Structure :default "None"))
  ;[0.15 1 0.15 0.5] Rotate Entire Tank
  (:Pressed
    (Utilities|FlowControl|Gate true) ; enters at Open
  )
  (:Released
    (Utilities|FlowControl|Gate true) ; enters at Close
  ))

(fn ConstructionScript)